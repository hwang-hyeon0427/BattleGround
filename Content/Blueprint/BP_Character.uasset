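; BP_Character is a player character with Enhanced Input movement, look, jump and a toggle between first- and third-person cameras.
; The view toggle swaps the active camera and hides the mesh from its owner in first person.
; Damage lowers health, and at zero or below Die increments the victim's death count and the killer's kill count on BP_PlayerState, then the killer's team tally on BP_GameState.
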(event Custom|Die
  (params (KillerController :type Controller%20Object%20Reference))
  (Utilities|FlowControl|Sequence
    (:then_0
      (bind _asbp_player_state (Utilities|Casting|CastToBP_PlayerState (Variables|GetPlayerState)))
      (Variables|/Game/Blueprint/BP_PlayerState.BP_PlayerState_C|SetDeathCount _asbp_player_state (+ (Variables|/Game/Blueprint/BP_PlayerState.BP_PlayerState_C|GetDeathCount _asbp_player_state) 1)))
    (:then_1
      (bind _asbp_player_state_2 (Utilities|Casting|CastToBP_PlayerState (Variables|/Script/Engine.Controller|GetPlayerState KillerController)))
      (Variables|/Game/Blueprint/BP_PlayerState.BP_PlayerState_C|SetKillCount _asbp_player_state_2 (+ (Variables|/Game/Blueprint/BP_PlayerState.BP_PlayerState_C|GetKillCount _asbp_player_state_2) 1))
      (bind _asbp_game_state (Utilities|Casting|CastToBP_GameState (Game|GetGameState)))
      (Variables|Default|SetAs%20BP%20Game%20State _asbp_game_state)
      (if (== (Variables|/Game/Blueprint/BP_PlayerState.BP_PlayerState_C|GetTeamId _asbp_player_state_2) 0)
        (Variables|/Game/Blueprint/BP_GameState.BP_GameState_C|SetTeamAKillCount (Variables|Default|GetAs%20BP%20Game%20State) (+ (Variables|/Game/Blueprint/BP_GameState.BP_GameState_C|GetTeamAKillCount (Variables|Default|GetAs%20BP%20Game%20State)) 1))
        (else
          (Variables|/Game/Blueprint/BP_GameState.BP_GameState_C|SetTeamBKillCount (Variables|Default|GetAs%20BP%20Game%20State) (+ (Variables|/Game/Blueprint/BP_GameState.BP_GameState_C|GetTeamBKillCount (Variables|Default|GetAs%20BP%20Game%20State)) 1)))))))

(event Input|EnhancedActionEvents|EnhancedInputActionIA_Move
  (params (ActionValue :type Vector%202D%20Structure) (ElapsedSeconds :type Float%20%28double-precision%29) (TriggeredSeconds :type Float%20%28double-precision%29) (InputAction :type Input%20Action%20Object%20Reference :default "/Game/Blueprint/IA_Move.IA_Move"))
  (bind _returnvalue (Pawn|GetControlRotation :!class /Script/Engine.Pawn))
  (Pawn|Input|AddMovementInput (Math|Vector|GetRightVector (Math|Rotator|MakeRotator 0.0 0.0 (.yaw _returnvalue))) (.x ActionValue) false)
  (Pawn|Input|AddMovementInput (Math|Vector|GetForwardVector (Math|Rotator|MakeRotator 0.0 0.0 (.yaw _returnvalue))) (.y ActionValue) false))

(event Input|EnhancedActionEvents|EnhancedInputActionIA_Rotation
  (params (ActionValue :type Vector%202D%20Structure) (ElapsedSeconds :type Float%20%28double-precision%29) (TriggeredSeconds :type Float%20%28double-precision%29) (InputAction :type Input%20Action%20Object%20Reference :default "/Game/Blueprint/IA_Rotation.IA_Rotation"))
  (Pawn|Input|AddControllerYawInput (.x ActionValue))
  (Pawn|Input|AddControllerPitchInput (.y ActionValue)))

(event Input|EnhancedActionEvents|EnhancedInputActionIA_Jump
  (params (ActionValue :type Boolean) (ElapsedSeconds :type Float%20%28double-precision%29) (TriggeredSeconds :type Float%20%28double-precision%29) (InputAction :type Input%20Action%20Object%20Reference :default "/Game/Blueprint/IA_Jump.IA_Jump"))
  (:Started
    (Character|Jump)))

(event Input|EnhancedActionEvents|EnhancedInputActionIA_ChangeView
  (params (ActionValue :type Boolean) (ElapsedSeconds :type Float%20%28double-precision%29) (TriggeredSeconds :type Float%20%28double-precision%29) (InputAction :type Input%20Action%20Object%20Reference :default "/Game/Blueprint/IA_ChangeView.IA_ChangeView"))
  (:Started
    (bind _output_get (Variables|Default|SetbIsFirstPerson? (not (Variables|Default|GetbIsFirstPerson?))))
    (if _output_get
      (Components|Activation|Activate (Variables|Default|GetFirstPersonCamera) false)
      (Components|Activation|Deactivate (Variables|Default|GetThirdPersonCamera))
      (Class|PrimitiveComponent|SetOwnerNoSee (Variables|Character|GetMesh) true)
      (else
        (Components|Activation|Activate (Variables|Default|GetThirdPersonCamera) false)
        (Components|Activation|Deactivate (Variables|Default|GetFirstPersonCamera))
        (Class|PrimitiveComponent|SetOwnerNoSee (Variables|Character|GetMesh) false)))))

(event EventBeginPlay
  (Input|AddMappingContext (PlayerController|LocalPlayerSubsystems|GetEnhancedInputLocalPlayerSubsystem (Game|GetPlayerController 0)) "/Game/Blueprint/IMC_Default.IMC_Default" 0 "(bIgnoreAllPressedKeysUntilRelease=True,bForceImmediately=False,bNotifyUserSettings=False)"))

(event Collision|EventActorBeginOverlap
  (params (OtherActor :type Actor%20Object%20Reference)))

(event EventTick
  (params (DeltaSeconds :type Float%20%28single-precision%29)))

(event Game|Damage|EventAnyDamage
  (params (Damage :type Float%20%28single-precision%29) (DamageType :type Damage%20Type%20Object%20Reference) (InstigatedBy :type Controller%20Object%20Reference) (DamageCauser :type Actor%20Object%20Reference))
  (bind _output_get (Variables|Default|SetCurrentHealth (- (Variables|Default|GetCurrentHealth) Damage)))
  (if (<= _output_get 0.0)
    (CallFunction|Die InstigatedBy)))

(fn ConstructionScript)